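; Actor component that feeds its owner's position to materials for interactive foliage in the ScifiJungle example player.
; Every tick it writes the owner's location, lowered by a Z offset, into the MPC_PlayerInteraction material parameter collection as the influencer position.
; It also pushes the effect radius and strength to the same collection, so any material reading it can react around the owner.
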(event EventBeginPlay)

(event EventTick
  (params (DeltaSeconds :type Float%20%28single-precision%29))
  ;[1 1 1] Foliage Interaction
  (Rendering|Material|SetVectorParameterValue "/Game/ScifiJungle/Materials/MMaterials/Functions/MPC_PlayerInteraction.MPC_PlayerInteraction" "InfluencerPosition" (Math|Conversions|ToLinearColor(Vector) (- (Transformation|GetActorLocation (Components|GetOwner self)) (* "0.000000,0.000000,1.000000" (Math|Conversions|ToVector(Float) (Variables|Default|GetEffectZOffset))))) :!class /Script/Engine.KismetMaterialLibrary)
  (Rendering|Material|SetScalarParameterValue "/Game/ScifiJungle/Materials/MMaterials/Functions/MPC_PlayerInteraction.MPC_PlayerInteraction" "EffectRadius" (Variables|Default|GetEffectRadius) :!class /Script/Engine.KismetMaterialLibrary)
  (Rendering|Material|SetScalarParameterValue "/Game/ScifiJungle/Materials/MMaterials/Functions/MPC_PlayerInteraction.MPC_PlayerInteraction" "Strenght" (Variables|Default|GetEffectStrenght) :!class /Script/Engine.KismetMaterialLibrary))